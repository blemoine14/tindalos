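; Hero character Blueprint that carries a weapon and shifts its camera rig toward the mouse cursor.
; The construction script snaps the Weapon component to the mesh's Weapon_r socket.
; Each tick it calls CalculateCameraPosition, then, if a mouse position is available, sets SpringArmRotator's relative location from the cursor's offset to viewport center.
; Screen vertical maps to inverted X and screen horizontal to Y, in unscaled pixels.
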(event EventBeginPlay)

(event Collision|EventActorBeginOverlap
  (params (OtherActor :type Actor%20Object%20Reference)))

(event EventTick
  (params (DeltaSeconds :type Float%20%28single-precision%29))
  (CallFunction|SetCameraPosition))

(fn ConstructionScript
  (Transformation|AttachComponentToComponent (Variables|Default|GetWeapon) (Variables|Character|GetMesh) "Weapon_r" "SnapToTarget" "SnapToTarget" "SnapToTarget" true))

(fn SetCameraPosition
  (bind _returnvalue (Game|GetPlayerController 0))
  (bind (_locationx _locationy _returnvalue_2) (Game|Player|GetMousePosition _returnvalue))
  (bind (_sizex _sizey) (HUD|GetViewportSize _returnvalue))
  (Class|HeroCharacter|CalculateCameraPosition)
  (if _returnvalue_2
    (Transformation|SetRelativeLocation (Variables|Default|GetSpringArmRotator) (Math|Vector|MakeVector (- (Math|Conversions|ToFloat(Integer) (/ _sizey 2)) _locationy) (- _locationx (Math|Conversions|ToFloat(Integer) (/ _sizex 2))) 0.0) false false)))