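; AI controller for enemies that runs the Ennemies_BT behavior tree on begin play.
; Every tick it writes the PlayerLocation blackboard key from the positions of player 0 and its controlled pawn.
; The stored point is the player's location offset toward the enemy, with horizontal distance divided by Sensibility and height matching the enemy's own.
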(event EventBeginPlay
  (AI|RunBehaviorTree "/Game/Blueprint/Ennemies/Ennemies_BT.Ennemies_BT"))

(event EventTick
  (params (DeltaSeconds :type Float%20%28single-precision%29))
  (bind _returnvalue (Game|Player|GetPlayerPawn 0))
  (bind _returnvalue_2 (Pawn|GetControlledPawn))
  (bind _returnvalue_3 (Transformation|GetActorLocation _returnvalue))
  (bind _returnvalue_4 (Transformation|GetActorLocation _returnvalue_2))
  (bind _returnvalue_5 (- _returnvalue_4 _returnvalue_3))
  (AI|Components|Blackboard|SetValueasVector (AI|GetBlackboard 0) (Variables|Default|GetPlayerLocation) (+ (Math|Vector|MakeVector (/ (.x _returnvalue_5) (Variables|Default|GetSensibility)) (/ (.y _returnvalue_5) (Variables|Default|GetSensibility)) (.z _returnvalue_5)) _returnvalue_3)))

(fn ConstructionScript)